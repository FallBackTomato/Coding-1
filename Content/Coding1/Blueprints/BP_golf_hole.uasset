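; Golf hole actor that detects a BP_golf_ball being holed and calls Win on BP_Sam.
; Capsule overlap records ball velocity and sets BallHoled; sphere overlap fires a RadialForce impulse every 0.1s until that flag is set.
; On cylinder hit, velocity-to-normal dot products gate success, though the 250 speed check compares a constant zero.
; A successful hit raises ball damping, then disables physics after half a second.
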(event OnComponentEndOverlap(Sphere)
  (params (OverlappedComponent :type Primitive%20Component%20Object%20Reference) (OtherActor :type Actor%20Object%20Reference) (OtherComp :type Primitive%20Component%20Object%20Reference) (OtherBodyIndex :type Integer))
  (Variables|Default|Setball_holed false))

(event OnComponentBeginOverlap(Sphere)
  (params (OverlappedComponent :type Primitive%20Component%20Object%20Reference) (OtherActor :type Actor%20Object%20Reference) (OtherComp :type Primitive%20Component%20Object%20Reference) (OtherBodyIndex :type Integer) (bFromSweep :type Boolean) (SweepResult :type Hit%20Result%20Structure%20%28by%20ref%29))
  (Development|PrintText "begin overlap")
  (Class|RadialForceComponent|FireImpulse (Variables|Default|GetRadialForce) :!label _label)
  (Utilities|FlowControl|Delay 0.1)
  (if (not (stale OnComponentBeginOverlap(Capsule) _output_get))
    (goto _label)))

(event OnComponentBeginOverlap(Capsule)
  (params (OverlappedComponent :type Primitive%20Component%20Object%20Reference) (OtherActor :type Actor%20Object%20Reference) (OtherComp :type Primitive%20Component%20Object%20Reference) (OtherBodyIndex :type Integer) (bFromSweep :type Boolean) (SweepResult :type Hit%20Result%20Structure%20%28by%20ref%29))
  (bind _asbp_golf_ball (Utilities|Casting|CastToBP_golf_ball OtherActor)) ; on hit golf ball
  (Variables|Default|Setball_vel (Transformation|GetComponentVelocity (Variables|/Game/Coding1/Blueprints/BP_golf_ball.BP_golf_ball_C|Getball _asbp_golf_ball)))
  (bind _output_get (Variables|Default|Setball_holed true)))

(event OnComponentHit(Cylinder)
  (params (HitComponent :type Primitive%20Component%20Object%20Reference) (OtherActor :type Actor%20Object%20Reference) (OtherComp :type Primitive%20Component%20Object%20Reference) (NormalImpulse :type Vector :default "0, 0, 0") (Hit :type Hit%20Result%20Structure%20%28by%20ref%29))
  (bind _impactnormal (Collision|BreakHitResult Hit))
  (bind _ball_vel (Variables|Default|Getball_vel))
  (bind _returnvalue (Math|Vector|Normalize _ball_vel))
  (bind _returnvalue_2 (Math|Vector|DotProduct _returnvalue _impactnormal))
  (bind _asbp_golf_ball (Utilities|Casting|CastToBP_golf_ball OtherActor))
  (if (and (> _returnvalue_2 0.85) (< 0.0 2.5e+02)) ; True if ball hits head on
    ;[0.15 0.15 0.15 0.5] set damping high
    (Class|PrimitiveComponent|SetLinearDamping (Variables|/Game/Coding1/Blueprints/BP_golf_ball.BP_golf_ball_C|Getball _asbp_golf_ball) 5.0 :!label _label)
    (Class|PrimitiveComponent|SetAngularDamping (Variables|/Game/Coding1/Blueprints/BP_golf_ball.BP_golf_ball_C|Getball _asbp_golf_ball) 5.0)
    (Utilities|FlowControl|Delay 0.5)
    (Physics|SetSimulatePhysics (Variables|/Game/Coding1/Blueprints/BP_golf_ball.BP_golf_ball_C|Getball _asbp_golf_ball) false) ; turn physics off
    (bind _returnvalue_3 (Actor|GetActorOfClass "/Game/Coding1/Blueprints/BP_Sam.BP_Sam_C"))
    (Default|Win _returnvalue_3)
    (elif (and (> _returnvalue_2 0.95) (< (Math|Vector|VectorLength (Variables|Default|Getball_vel)) 7.5e+02))
      (goto _label))))

(fn ConstructionScript)